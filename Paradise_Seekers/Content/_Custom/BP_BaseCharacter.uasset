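; Base character Blueprint that drives combat abilities through the Gameplay Ability System.
; BeginPlay grants each class in Abilities and adds a loose attack gameplay tag.
; Attack and dodge inputs activate abilities by their current tag variables, so setters like SetDodgeTag can swap the ability behind an input.
; Move, jump and numbered ability inputs are empty, and the tag setters other than dodge store nothing.
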(event Input|EnhancedActionEvents|EnhancedInputActionIA_Attack
  (params (ActionValue :type Boolean) (ElapsedSeconds :type Float%20%28double-precision%29) (TriggeredSeconds :type Float%20%28double-precision%29) (InputAction :type Input%20Action%20Object%20Reference :default "/Game/_Custom/Input/Actions/IA_Attack.IA_Attack"))
  (:Started
    (CallFunction|AttackClick)))

(event Input|EnhancedActionEvents|EnhancedInputActionIA_Move
  (params (ActionValue :type Vector%202D%20Structure) (ElapsedSeconds :type Float%20%28double-precision%29) (TriggeredSeconds :type Float%20%28double-precision%29) (InputAction :type Input%20Action%20Object%20Reference :default "/Game/_Custom/Input/Actions/IA_Move.IA_Move")))

(event Input|EnhancedActionEvents|EnhancedInputActionIA_Dodge
  (params (ActionValue :type Boolean) (ElapsedSeconds :type Float%20%28double-precision%29) (TriggeredSeconds :type Float%20%28double-precision%29) (InputAction :type Input%20Action%20Object%20Reference :default "/Game/_Custom/Input/Actions/IA_Dodge.IA_Dodge"))
  (:Started
    (CallFunction|DodgeClick)))

(event Input|EnhancedActionEvents|EnhancedInputActionIA_Ability1
  (params (ActionValue :type Boolean) (ElapsedSeconds :type Float%20%28double-precision%29) (TriggeredSeconds :type Float%20%28double-precision%29) (InputAction :type Input%20Action%20Object%20Reference :default "/Game/_Custom/Input/Actions/IA_Ability1.IA_Ability1")))

(event Input|EnhancedActionEvents|EnhancedInputActionIA_Ability2
  (params (ActionValue :type Boolean) (ElapsedSeconds :type Float%20%28double-precision%29) (TriggeredSeconds :type Float%20%28double-precision%29) (InputAction :type Input%20Action%20Object%20Reference :default "/Game/_Custom/Input/Actions/IA_Ability2.IA_Ability2")))

(event Input|EnhancedActionEvents|EnhancedInputActionIA_Ability3
  (params (ActionValue :type Boolean) (ElapsedSeconds :type Float%20%28double-precision%29) (TriggeredSeconds :type Float%20%28double-precision%29) (InputAction :type Input%20Action%20Object%20Reference :default "/Game/_Custom/Input/Actions/IA_Ability3.IA_Ability3")))

(event Input|EnhancedActionEvents|EnhancedInputActionIA_Jump
  (params (ActionValue :type Boolean) (ElapsedSeconds :type Float%20%28double-precision%29) (TriggeredSeconds :type Float%20%28double-precision%29) (InputAction :type Input%20Action%20Object%20Reference :default "/Game/_Custom/Input/Actions/IA_Jump.IA_Jump")))

(event EventBeginPlay
  (for _array_element (Variables|Default|GetAbilities)
    (GameplayAbilities|GiveAbility (Variables|Default|GetAbilitySystem) _array_element 0 -1)
    (Ability|GameplayEffect|AddLooseGameplayTags self (GameplayTags|MakeLiteralGameplayTagContainer "(GameplayTags=((TagName=\"Abilities.EKRY.Attack.A1\")))"))))

(event Collision|EventActorBeginOverlap
  (params (OtherActor :type Actor%20Object%20Reference)))

(event EventTick
  (params (DeltaSeconds :type Float%20%28single-precision%29)))

(fn ConstructionScript)

(fn AttackClick
  (Abilities|TryActivateAbilitiesbyTag (Variables|Default|GetAbilitySystem) (GameplayTags|MakeGameplayTagContainerfromTag (Variables|Default|GetCurrentNormalAttackAbility)) true))

(fn DodgeClick
  (bind _currentdodge (Variables|Default|GetCurrentDodge))
  (Development|PrintString (GameplayTags|GetDebugStringfromGameplayTag _currentdodge))
  (Abilities|TryActivateAbilitiesbyTag (Variables|Default|GetAbilitySystem) (GameplayTags|MakeGameplayTagContainerfromTag _currentdodge) true)
  (CallFunction|SetDodgeTag))

(fn SetBasicTag
  (params (Tag :type Gameplay%20Tag%20Structure))
  (if (!= Tag "")
    _))

(fn SetDodgeTag
  (params (Tag :type Gameplay%20Tag%20Structure))
  (if (!= Tag "")
    (Variables|Default|SetCurrentDodge Tag)))

(fn SetExpiryTime
  (params (Tag :type Gameplay%20Tag%20Structure) (MaxTime :type Float%20%28double-precision%29) (ChainAfter :type Boolean%20%28by%20ref%29))
  (return false))

(fn SetJumpTag
  (params (Tag :type Gameplay%20Tag%20Structure))
  (if (!= Tag "")
    (return Tag)))

(fn SetS1Tag
  (params (Tag :type Gameplay%20Tag%20Structure))
  (if (!= Tag "")
    (return Tag)))

(fn SetS2Tag
  (params (Tag :type Gameplay%20Tag%20Structure))
  (if (!= Tag "")
    (return Tag)))

(fn SetS3Tag
  (params (Tag :type Gameplay%20Tag%20Structure))
  (if (!= Tag "")
    (return Tag)))